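; BP_Turret1 is a turret that shoots at the player's third-person character when its PawnSensing component sees it.
; On sight it snaps its whole actor rotation toward the pawn, then after a short delay spawns a BP_Bullet at its Arrow component.
; The bullet receives an impulse along the turret's forward vector, scaled by FireStrength.
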(event OnSeePawn(PawnSensing)
  (params (Pawn :type Pawn%20Object%20Reference))
  (Utilities|Casting|CastToBP_ThirdPersonCharacter Pawn)
  (Transformation|SetActorRotation (Math|Rotator|FindLookatRotation (Transformation|GetActorLocation) (Transformation|GetActorLocation Pawn)))
  (Utilities|FlowControl|Delay 0.2)
  (Game|SpawnActorfromClass "/Game/Asian_Village/blueprints/BP_Bullet.BP_Bullet_C" (Transformation|GetWorldTransform (Variables|Default|GetArrow)) "Undefined" "MultiplyWithRoot" 0 (* (Transformation|GetActorForwardVector) (Variables|Default|GetFire%20Strength)) 0))

(fn ConstructionScript)