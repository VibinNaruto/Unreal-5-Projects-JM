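; BP_Switch is a light switch that toggles a referenced rect light when interacted with.
; Each Interact event plays the Explosion01 sound in 2D, flips the IsLightOn flag and prints the new state on screen.
; It switches the light by setting the intensity of its RectLightComponent to a fixed brightness or to zero, rather than changing its visibility.
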(event EventInteract
  (bind _light (Variables|Default|Getlight))
  (bind _rectlightcomponent (Variables|/Script/Engine.RectLight|GetRectLightComponent _light))
  (Audio|PlaySound2D "/Game/StarterContent/Audio/Explosion01.Explosion01" 1.0 1.0 0.0 0 0)
  (if (not (Variables|Default|GetisLightOn))
    (Variables|Default|SetisLightOn true)
    (Development|PrintString "Turn Light On")
    (Rendering|Components|Light|SetIntensity _rectlightcomponent 8e+01)
    (else
      (Variables|Default|SetisLightOn false)
      (Development|PrintString "Turn Light Off")
      (Rendering|Components|Light|SetIntensity _rectlightcomponent 0.0))))

(fn ConstructionScript)