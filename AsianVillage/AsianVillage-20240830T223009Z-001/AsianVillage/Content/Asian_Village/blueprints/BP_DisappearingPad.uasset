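; BP_DisappearingPad is a platform that vanishes shortly after the player character touches it and later returns.
; Box overlap by BP_ThirdPersonCharacter sets the Pad's material, then after a short delay hides it and disables collision.
; Any end overlap on the Box starts a longer delay, then sets the material again and restores visibility and collision.
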(event OnComponentBeginOverlap(Box)
  (params (OverlappedComponent :type Primitive%20Component%20Object%20Reference) (OtherActor :type Actor%20Object%20Reference) (OtherComp :type Primitive%20Component%20Object%20Reference) (OtherBodyIndex :type Integer) (bFromSweep :type Boolean) (SweepResult :type Hit%20Result%20Structure%20%28by%20ref%29))
  (Utilities|Casting|CastToBP_ThirdPersonCharacter OtherActor)
  (Rendering|Material|SetMaterial (Variables|Default|GetPad) 0 0)
  (Utilities|FlowControl|Delay 1.0)
  (Rendering|SetVisibility (Variables|Default|GetPad) false false)
  (Collision|SetCollisionEnabled (Variables|Default|GetPad) "NoCollision"))

(event OnComponentEndOverlap(Box)
  (params (OverlappedComponent :type Primitive%20Component%20Object%20Reference) (OtherActor :type Actor%20Object%20Reference) (OtherComp :type Primitive%20Component%20Object%20Reference) (OtherBodyIndex :type Integer))
  (Utilities|FlowControl|Delay 3.0)
  (Rendering|Material|SetMaterial (Variables|Default|GetPad) 0 0)
  (Rendering|SetVisibility (Variables|Default|GetPad) true false)
  (Collision|SetCollisionEnabled (Variables|Default|GetPad) "QueryAndPhysics"))

(fn ConstructionScript)