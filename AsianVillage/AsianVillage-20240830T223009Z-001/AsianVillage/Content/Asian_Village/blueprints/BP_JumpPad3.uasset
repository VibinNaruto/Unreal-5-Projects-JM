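; BP_JumpPad3 is a jump pad that launches the third-person player character along the pad's up direction.
; When the character overlaps the Box, it waits for a configurable delay, then adds an impulse to the character's movement component.
; The impulse follows the normalized up vector of the JumpPad component's world rotation, scaled by Power, so tilting the pad aims the launch.
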(event OnComponentBeginOverlap(Box)
  (params (OverlappedComponent :type Primitive%20Component%20Object%20Reference) (OtherActor :type Actor%20Object%20Reference) (OtherComp :type Primitive%20Component%20Object%20Reference) (OtherBodyIndex :type Integer) (bFromSweep :type Boolean) (SweepResult :type Hit%20Result%20Structure%20%28by%20ref%29))
  (bind _power (Variables|Default|GetPower))
  (bind _jumppad (Variables|Default|GetJumpPad))
  (bind _returnvalue (Transformation|GetWorldRotation _jumppad))
  (bind _returnvalue_2 (* _power 1.5e+03))
  (bind _returnvalue_3 (Math|Vector|GetUpVector _returnvalue))
  (bind _returnvalue_4 (Math|Vector|Normalize _returnvalue_3))
  (bind _asbp_third_person_character (Utilities|Casting|CastToBP_ThirdPersonCharacter OtherActor))
  (Utilities|FlowControl|Delay (Variables|Default|GetImpulse%20Delay))
  (Physics|AddImpulse (Variables|/Script/Engine.Character|GetCharacterMovement _asbp_third_person_character) (Math|Vector|MakeVector (* (.x _returnvalue_4) _returnvalue_2) (* (.y _returnvalue_4) _returnvalue_2) (* (.z _returnvalue_4) _returnvalue_2)) false))

(fn ConstructionScript)