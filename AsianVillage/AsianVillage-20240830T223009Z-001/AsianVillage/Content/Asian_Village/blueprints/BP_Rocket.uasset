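; BP_Rocket is a homing rocket projectile actor that explodes on impact.
; On BeginPlay it plays a launch sound and sets the MissuleTarget variable as the homing target of its ProjectileMovement component.
; When its Box component hits something, it fires a RadialForce impulse, spawns an explosion particle and sound at the hit location, then destroys itself after a short delay.
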(event OnComponentHit(Box)
  (params (HitComponent :type Primitive%20Component%20Object%20Reference) (OtherActor :type Actor%20Object%20Reference) (OtherComp :type Primitive%20Component%20Object%20Reference) (NormalImpulse :type Vector :default "0, 0, 0") (Hit :type Hit%20Result%20Structure%20%28by%20ref%29))
  (bind _location (Collision|BreakHitResult Hit))
  (Class|RadialForceComponent|FireImpulse (Variables|Default|GetRadialForce))
  (Effects|SpawnEmitteratLocation "/Game/MilitaryWeapDark/FX/P_RocketLauncher_Explosion_01.P_RocketLauncher_Explosion_01" _location)
  (Audio|PlaySoundatLocation "/Game/MilitaryWeapDark/Sound/RocketLauncher/wavs/RocketLauncher_Explosion01.RocketLauncher_Explosion01" _location "0, 0, 0" 1.0 1.0 0.0 0 0 0 0)
  (Utilities|FlowControl|Delay 0.2)
  (Actor|DestroyActor))

(event EventBeginPlay
  (Audio|PlaySoundatLocation "/Game/MilitaryWeapDark/Sound/RocketLauncher/wavs/RocketLauncherB_Fire01.RocketLauncherB_Fire01" (Transformation|GetActorLocation) "0, 0, 0" 1.0 1.0 0.0 0 0 0 0)
  (Variables|/Script/Engine.ProjectileMovementComponent|SetHomingTargetComponent (Variables|Default|GetProjectileMovement) (Variables|Default|GetmissuleTarget)))

(event Collision|EventActorBeginOverlap
  (params (OtherActor :type Actor%20Object%20Reference)))

(event EventTick
  (params (DeltaSeconds :type Float%20%28single-precision%29)))

(fn ConstructionScript)