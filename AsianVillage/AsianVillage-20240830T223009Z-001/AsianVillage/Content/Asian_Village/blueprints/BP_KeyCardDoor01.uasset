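; BP_KeyCardDoor01 is a door that the player can swing open and closed only while holding the white key card.
; On BeginPlay it caches the player character, and its Interactt event checks the WhiteKeyCard flag in that character's KeyCards.
; A FlipFlop alternately plays and reverses a Timeline that lerps the door's relative yaw for the swing.
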(event EventBeginPlay
  (bind _asbp_third_person_character (Utilities|Casting|CastToBP_ThirdPersonCharacter (Game|GetPlayerCharacter 0)))
  (Variables|Default|SetAs%20BP%20Third%20Person%20Character _asbp_third_person_character))

(event EventInteractt
  (if (.WhiteKeyCard (Utilities|Struct|BreakKeyCards (Variables|/Game/ThirdPerson/Blueprints/BP_ThirdPersonCharacter.BP_ThirdPersonCharacter_C|GetKeyCards (Variables|Default|GetAs%20BP%20Third%20Person%20Character))))
    (Utilities|FlowControl|FlipFlop
      (:A
        (bind _newtrack_0 (Timeline|Timeline Play)
          (:Update
            (Transformation|SetRelativeRotation (Variables|Default|GetDoor) (Math|Rotator|MakeRotator 0.0 0.0 (Math|Float|Lerp 0.0 -1e+02 _newtrack_0)) false false))))
      (:B
        (Timeline|Timeline Reverse)))))

(fn ConstructionScript)