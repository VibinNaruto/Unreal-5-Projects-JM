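; BP_PressureDoor is a door that moves vertically when enough pressure switches are active.
; SwitchActivated and SwitchDeActivated events raise and lower a count of active switches, then compare it to the required number.
; Meeting the threshold plays the DoorActivation timeline, otherwise it reverses, with the timeline's value setting the Door's relative Z location.
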(event Custom|SwitchActivated
  (Math|Integer|IncrementInt (Variables|Default|GetPressureSwitchesActive)
    (:%20%20
      (if (>= (Variables|Default|GetPressureSwitchesActive) (Variables|Default|GetPressureSwitchesNeeded))
        (bind _doorpostion (Timeline|DoorActivation Play)
          (:Update
            (Transformation|SetRelativeLocation (Variables|Default|GetDoor) (Math|Vector|MakeVector 0.0 0.0 _doorpostion) false false)))
        (else
          (Timeline|DoorActivation Reverse))))))

(event Custom|SwitchDeActivated
  (Math|Integer|DecrementInt (Variables|Default|GetPressureSwitchesActive)
    (:%20%20
      (if (>= (Variables|Default|GetPressureSwitchesActive) (Variables|Default|GetPressureSwitchesNeeded))
        (bind _doorpostion (Timeline|DoorActivation Play)
          (:Update
            (Transformation|SetRelativeLocation (Variables|Default|GetDoor) (Math|Vector|MakeVector 0.0 0.0 _doorpostion) false false)))
        (else
          (Timeline|DoorActivation Reverse))))))

(fn ConstructionScript)